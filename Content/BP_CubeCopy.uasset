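; BP_CubeCopy is an actor that spawns a row of five Cube_Blueprint cubes on BeginPlay, apparently a test of arrays and random materials.
; Each cube is spaced along X, stored in AllCubes and given a random material, though RandomInteger(4) never selects Mat4.
; A second loop compares cube references, not materials, against FirstMaterial (the last cube spawned), clearing Done on mismatch and printing debug messages.
; UpdateMaterial is an empty stub.
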(event `self.ReceiveBeginPlay`
  (for _index (range 5)
    (bind _returnvalue (`|SpawnActorFromClass` "/Game/Cube_Blueprint.Cube_Blueprint_C" (`KismetMathLibrary.MakeTransform` (+ (`KismetMathLibrary.MakeVector` (* _index (`self.SpaceBetweeen`))) (`KismetMathLibrary.MakeVector` 1300.0 300.0 200.0))) "Undefined" "MultiplyWithRoot" null null))
    (bind _returnvalue_2 (`KismetArrayLibrary.Array_Add` (`self.AllCubes`) _returnvalue))
    (`KismetSystemLibrary.PrintString` (`KismetStringLibrary.Conv_IntToString` _returnvalue_2))
    (switch `int` (`KismetMathLibrary.RandomInteger` 4)
      (:`0`
        (bind _staticmeshcomponent (`StaticMeshActor.StaticMeshComponent` _returnvalue))
        (`PrimitiveComponent.SetMaterial` _staticmeshcomponent 0 (`self.Mat_0`)))
      (:`1`
        (`PrimitiveComponent.SetMaterial` _staticmeshcomponent 0 (`self.Mat_1`)))
      (:`2`
        (`PrimitiveComponent.SetMaterial` _staticmeshcomponent 0 (`self.Mat_2`)))
      (:`3`
        (`PrimitiveComponent.SetMaterial` _staticmeshcomponent 0 (`self.Mat_3`)))
      (:`4`
        (`PrimitiveComponent.SetMaterial` _staticmeshcomponent 0 (`self.Mat_4`)))))
  (set `self.FirstMaterial` _returnvalue)
  (for _array_element (`self.AllCubes`)
    (if (== _array_element (`self.FirstMaterial`))
      (`KismetSystemLibrary.PrintString` "an element matches firsat materialHello")
      (else
        (set `self.Done` false))))
  (if (`self.Done`)
    (`KismetSystemLibrary.PrintString` "Returned true")))

(fn `UpdateMaterial`)

(fn `UserConstructionScript`)